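; BP_DoorManager keeps a map of BP_Door actors and toggles one by corridor, room and door index.
; MakeDoorKey combines the indices into a string key, which ToggleDoorByIndices looks up before calling ToggleDoor, printing a message if missing.
; RegisterDoor adds a given key and door to the map.
; An EventGraph loop meant to register every level door is not connected to any event, so it never runs.
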(fn ConstructionScript)

(fn MakeDoorKey
  (params (CorridorIndex :type Integer) (RoomIndex :type Integer) (DoorIndex :type Integer))
  (return (Utilities|String|Append "C" (Utilities|String|ToString(Integer) CorridorIndex) "_R" (Utilities|String|ToString(Integer) RoomIndex) "_D" (Utilities|String|ToString(Integer) DoorIndex))))

(fn RegisterDoor
  (params (Key :type String) (DoorRef :type BP%20Door%20Object%20Reference))
  (Utilities|Map|Add (Variables|Default|GetDoorMap) Key DoorRef)
  (Development|PrintString "\"Registered: \" + Key"))

(fn ToggleDoorbyIndices
  (params (CorridorIndex :type Integer) (RoomIndex :type Integer) (DoorIndex :type Integer))
  (bind _key (CallFunction|MakeDoorKey CorridorIndex RoomIndex DoorIndex))
  (if (.ReturnValue (Utilities|Map|Find (Variables|Default|GetDoorMap) _key))
    (Default|ToggleDoor (.Value (Utilities|Map|Find (Variables|Default|GetDoorMap) _key)))
    (else
      (Development|PrintString "\"Door not found: \" + Key"))))