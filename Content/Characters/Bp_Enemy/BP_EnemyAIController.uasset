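; AI controller for the enemy that feeds patrol and perception data to the BB_Enemy blackboard.
; BeginPlay runs BT_Enemy only if PatrolPoints has entries, but the loop's "Patrol"-tag filter that would fill it is disconnected.
; Perception updates set the target and last known location on sensing.
; Losing a stimulus stores its location and starts a short forget timer, apparently meant for ForgetTarget, which clears TargetActor.
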(event OnTargetPerceptionUpdated(AIPerception)
  (params (Actor :type Actor%20Object%20Reference) (Stimulus :type AI%20Stimulus%20Structure))
  (bind (_age _expirationage _strength _stimuluslocation _receiverlocation _tag _bsuccessfullysensed) (Utilities|Struct|BreakAIStimulus Stimulus))
  (bind _bbcomp (Variables|Default|GetBBComp))
  (if _bsuccessfullysensed
    (Utilities|Time|ClearandInvalidateTimerbyHandle (Variables|Default|GetForgetHandle))
    (AI|Components|Blackboard|SetValueasObject _bbcomp (Utilities|Name|MakeLiteralName "TargetActor") Actor)
    (AI|Components|Blackboard|SetValueasVector _bbcomp (Utilities|Name|MakeLiteralName "LastKnownLocation") (Transformation|GetActorLocation Actor))
    (else
      (Utilities|Time|ClearandInvalidateTimerbyHandle (Variables|Default|GetForgetHandle))
      (AI|Components|Blackboard|SetValueasVector (Variables|Default|GetBBComp) (Utilities|Name|MakeLiteralName "LastKnownLocation") _stimuluslocation)
      (bind _returnvalue (Utilities|Time|SetTimerbyEvent (EventDispatchers|CreateEvent :!event Custom|ForgetTarget) 3.0))
      (Variables|Default|SetForgetHandle _returnvalue))))

(event Custom|ForgetTarget
  (AI|Components|Blackboard|SetValueasObject (Variables|Default|GetBBComp) (Utilities|Name|MakeLiteralName "TargetActor") 0))

(event EventBeginPlay
  (bind _blackboardcomponent (Class|AIController|UseBlackboard "/Game/Characters/Bp_Enemy/BB_Enemy.BB_Enemy"))
  (Variables|Default|SetBBComp _blackboardcomponent)
  (Actor|GetAllActorsOfClass "/Script/Engine.TargetPoint")
  (for _array_element 0
    _)
  (if (> (Utilities|Array|Length (Variables|Default|GetPatrolPoints)) 0)
    (Class|BlackboardComponent|SetValueasInt (Variables|Default|GetBBComp) (Utilities|Name|MakeLiteralName "PatrolIndex"))
    (AI|Components|Blackboard|SetValueasObject (Variables|Default|GetBBComp) (Utilities|Name|MakeLiteralName "PatrolPoint") (Utilities|Array|Get(acopy) (Variables|Default|GetPatrolPoints)))
    (AI|RunBehaviorTree "/Game/Characters/Bp_Enemy/BT_Enemy.BT_Enemy")))

(fn ConstructionScript)

(fn BPEnemyAIControllerAutoGenFunc)